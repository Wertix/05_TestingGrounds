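; BP_Tile is a terrain tile for an infinite terrain system, with a barrier that the player unlocks by entering its trigger box.
; The barrier starts solid and red, turns passable and green on player overlap, and relocks on exit.
; Exiting also tells InfiniteTerrainGameMode to spawn and remove a tile.
; An Arrow component supplies the attach transform through GetAttachLocation.
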(event `self.ReceiveBeginPlay`
  (`self.LockBarrier`))

(event `self.Box.OnComponentBeginOverlap`
  (params (OverlappedComponent :type "PrimitiveComponent Object Reference") (OtherActor :type "Actor Object Reference") (OtherComp :type "PrimitiveComponent Object Reference") (OtherBodyIndex :type Integer) (bFromSweep :type Boolean) (SweepResult :type "HitResult Structure (by ref)"))
  (`self.IsPlayerActor` OtherActor)
  (`self.UnlockBarrier`))

(event `self.Box.OnComponentEndOverlap`
  (params (OverlappedComponent :type "PrimitiveComponent Object Reference") (OtherActor :type "Actor Object Reference") (OtherComp :type "PrimitiveComponent Object Reference") (OtherBodyIndex :type Integer))
  (bind _asinfinite_terrain_game_mode (cast `/Game/Dynamic/InfiniteTerrainGameMode` (`GameplayStatics.GetGameMode`) :!pure true))
  (`self.IsPlayerActor` OtherActor)
  (`self.LockBarrier`)
  (`/Game/Dynamic/InfiniteTerrainGameMode.SpawnTile` _asinfinite_terrain_game_mode)
  (`/Game/Dynamic/InfiniteTerrainGameMode.RemoveTile` _asinfinite_terrain_game_mode))

(fn `GetAttachLocation`
  (returns (AttachTransform :type "Transform Structure"))
  (return (`SceneComponent.K2_GetComponentToWorld` (`self.Arrow`))))

(fn `LockBarrier`
  (`PrimitiveComponent.SetCollisionEnabled` (`self.Barrier`) "QueryAndPhysics")
  (`PrimitiveComponent.SetMaterial` (`self.Barrier`) 0 "/Game/Dynamic/Terrain/MI_RedBarrier.MI_RedBarrier"))

(fn `UnlockBarrier`
  (`PrimitiveComponent.SetCollisionEnabled` (`self.Barrier`) "NoCollision")
  (`PrimitiveComponent.SetMaterial` (`self.Barrier`) 0 "/Game/Dynamic/Terrain/MI_GreenBarrier.MI_GreenBarrier"))

(fn `UserConstructionScript`)